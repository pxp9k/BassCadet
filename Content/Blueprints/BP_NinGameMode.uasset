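; Game mode that opens the lead sheet editor UI when play begins.
; BeginPlay creates the editor widget, adds it to the viewport and shows the first player's mouse cursor; a UI-only input mode call exists but never runs.
; Similar helper functions create the main UI and session browser widgets, though nothing in this Blueprint calls them.
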(event EventBeginPlay
  (CallFunction|CreateLeadSheetEditorWidget))

(event EventTick
  (params (DeltaSeconds :type Float%20%28single-precision%29)))

(fn ConstructionScript)

(fn CreateMainUIWidget
  (bind _returnvalue (UserInterface|CreateWidget "/Game/UI/Main/UI_MainW.UI_MainW_C"))
  (UserInterface|Viewport|AddtoViewport _returnvalue 0))

(fn CreateSessionBrowserWidget
  (bind _returnvalue (UserInterface|CreateWidget "/Game/UI/SessionBrowser/UI_SessionBrowserW.UI_SessionBrowserW_C"))
  (UserInterface|Viewport|AddtoViewport _returnvalue 0))

(fn CreateLeadSheetEditorWidget
  (bind _returnvalue (UserInterface|CreateWidget "/Game/UI/LeadSheetEditor/UI_LeadSheetEditorW.UI_LeadSheetEditorW_C"))
  (UserInterface|Viewport|AddtoViewport _returnvalue 0)
  (Variables|/Script/Engine.PlayerController|SetbShowMouseCursor (Game|GetPlayerController 0) true))