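; NinJam-style jam actor that keeps time at 85 BPM, starts a matching 16 BPI audio track and highlights the current bar on a chord grid.
; On each beat it moves the grid widget highlight to the current bar and, if Click is on, plays a high or low metronome click.
; The track fires on the first beat of bar one.
; DisplayChord is an empty stub.
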(event EventBeginPlay
  (Class|NinJam|SetBPM 85))

(event Collision|EventActorBeginOverlap
  (params (OtherActor :type Actor%20Object%20Reference)))

(event EventTick
  (params (DeltaSeconds :type Float%20%28single-precision%29)))

(event EventOnBeat
  (bind _currentbar (Variables|Default|GetCurrentBar))
  (CallFunction|HighlightBar _currentbar)
  (Variables|Default|SetLastHighlightedBeat _currentbar)
  (if (== (Variables|Default|GetCurrentBeat) 1)
    (if (Variables|Default|GetbClick)
      (Audio|PlaySound2D "/Game/Sounds/Click/MetroClick_High_Cue.MetroClick_High_Cue" 1.0 1.0 0.0 0 0))
    (if (== (Variables|Default|GetCurrentBar) 1)
      (Audio|PlaySound2D "/Game/Sounds/16Bar_85bpm/16BPI_85_bpm.16BPI_85_bpm" 1.0 1.0 0.0 0 0))
    (elif (Variables|Default|GetbClick)
      (Audio|PlaySound2D "/Game/Sounds/Click/MetroClick_Low_Cue.MetroClick_Low_Cue" 1.0 1.0 0.0 0 0))))

(fn ConstructionScript)

(fn HighlightBar
  (params (BarNumber :type Integer))
  (Default|SetHighlightOFF (Variables|Default|GetChordGridWPtr) (Variables|Default|GetLastHighlightedBeat))
  (Default|SetHighlightON (Variables|Default|GetChordGridWPtr) BarNumber))

(fn DisplayChord)