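; Player controller that finds the BP_NinJam actor on BeginPlay and toggles its Click flag from the ClickToggle input action.
; Two helper functions convert MIDI note numbers to sharp or flat note names by indexing name arrays, offset from note 21 and wrapped every 12.
; An unconnected FlipFlop holds logic to show or hide a UI_Sequencer widget while switching input mode and mouse cursor visibility.
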(event EventBeginPlay
  (bind _outactors (Actor|GetAllActorsOfClass "/Game/Blueprints/BP_NinJam.BP_NinJam_C"))
  (Variables|Default|SetNinJam (Utilities|Array|Get(acopy) _outactors)))

(event EventTick
  (params (DeltaSeconds :type Float%20%28single-precision%29)))

(event Input|ActionEvents|InputActionClickToggle
  (params (Key :type Key%20Structure :default "None"))
  (bind _ninjam (Variables|Default|GetNinJam))
  (:Pressed
    (Variables|/Script/NinSession.NinJam|SetbClick _ninjam (not (Variables|/Script/NinSession.NinJam|GetbClick _ninjam)))))

(fn ConstructionScript)

(fn Midi2NoteStringSharp
  (params (MidiNote :type Integer))
  (return (Utilities|Array|Get(acopy) (Variables|Default|GetNotesSharp) (Math|Integer|%(Integer) (- MidiNote 21) 12))))

(fn Midi2NoteStringFlat
  (params (MidiNote :type Integer))
  (return (Utilities|Array|Get(acopy) (Variables|Default|GetNotesFlat) (Math|Integer|%(Integer) (- MidiNote 21) 12))))