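; BP_Pulsor is a metronome actor that keeps a musical pulse, tracking bar and beat position at a set BPM.
; Tick accumulates delta time against the beat length, carrying the remainder over, and rolls into a new bar once the beat passes BPI.
; Each beat can play a high or low click, with the high one marking beat one.
; It also prints debug timing and fetches the player controller's sequencer widget at startup.
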(event EventBeginPlay
  (CallFunction|GetUIWidget)
  (CallFunction|SetBPM (Variables|Default|GetBPM)))

(event Collision|EventActorBeginOverlap
  (params (OtherActor :type Actor%20Object%20Reference)))

(event EventTick
  (params (DeltaSeconds :type Float%20%28single-precision%29))
  (CallFunction|ProcessTimeUpdate DeltaSeconds)
  (CallFunction|UpdateDebugInfo))

(fn ConstructionScript)

(fn CalculateNTime
  ;[1 1 1] Calculate time for each beat in seconds (the time one beat takes)
  (Variables|Default|SetNTime (/ 6e+01 (Variables|Default|GetBPM))))

(fn ProcessTimeUpdate
  (params (DeltaTime :type Float%20%28single-precision%29))
  (bind _ntime (Variables|Default|GetNTime))
  (bind _output_get (Variables|Default|SetCurrentNTime (+ (Variables|Default|GetCurrentNTime) DeltaTime)))
  (if (>= _output_get _ntime)
    (Variables|Default|SetCurrentNTime (- _output_get _ntime))
    (CallFunction|CountBeat)))

(fn CountBeat
  (bind _result (Math|Integer|IncrementInt (Variables|Default|GetBeat))
    (:%20%20
      (if (> _result (Variables|Default|GetBPI))
        (Math|Integer|IncrementInt (Variables|Default|GetBar)
          (:%20%20
            (Variables|Default|SetBeat 1)
            (CallFunction|OnOne)))
        (else
          (Variables|Default|SetBeat _result)))
      (CallFunction|PlayClickSound))))

(fn GetUIWidget
  (bind _asbp_player_controller (Utilities|Casting|CastToBP_PlayerController (Game|GetPlayerController 0)))
  (bind _output_get (Variables|Default|SetSequencerUIWidget (Variables|/Game/BP_PlayerController.BP_PlayerController_C|GetSequencerWidget _asbp_player_controller)))
  (return _output_get))

(fn SetBPM
  (params (NewBPMValuie :type Float%20%28single-precision%29))
  (Variables|Default|SetBPM NewBPMValuie)
  (CallFunction|CalculateNTime))

(fn UpdateDebugInfo
  (Development|PrintString (Utilities|String|Append "BPM: " (Utilities|String|ToString(Float) (Variables|Default|GetBPM)) " 
BPI: " (Utilities|String|ToString(Integer) (Variables|Default|GetBPI)) " / " (Utilities|String|ToString(Integer) (Variables|Default|GetNths)) " 
NTime = " (Utilities|String|ToString(Float) (Variables|Default|GetNTime)) " Sec. 
Bar / Beat: " (Utilities|String|ToString(Integer) (Variables|Default|GetBar)) " / " (Utilities|String|ToString(Integer) (Variables|Default|GetBeat))) true true "(R=1.000000,G=1.000000,B=1.000000,A=1.000000)" 0.0))

(fn PlayClickHigh
  (Audio|PlaySound2D "/Game/Sounds/Click/MetroClick_High_Cue.MetroClick_High_Cue" 1.0 1.0 0.0 0 0))

(fn PlayClickLow
  (Audio|PlaySound2D "/Game/Sounds/Click/MetroClick_Low_Cue.MetroClick_Low_Cue" 1.0 1.0 0.0 0 0))

(fn PlayClickSound
  (if (Variables|Default|GetClickSoundOn)
    (if (== (Variables|Default|GetBeat) 1)
      (CallFunction|PlayClickHigh)
      (else
        (CallFunction|PlayClickLow)))))

(fn OnOne
  (Development|PrintString "ONE!"))